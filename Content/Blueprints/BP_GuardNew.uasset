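; BP_GuardNew is a guard AI pawn that patrols four locations and reacts to seen pawns.
; GuardPatrol chains AI moves through the location array, pausing after each arrival and wrapping the index.
; On sight it faces the player and issues an AIMoveTo with no destination or target set, then a retriggerable delay resumes patrol.
; StartRotating, FinishRotation and StopChase are empty or unwired stubs.
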(event `self.ReceiveBeginPlay`
  (set `self.State` "NewEnumerator0")
  (`self.GuardPatrol`))

(event `self.ReceiveTick`
  (params (DeltaSeconds :type "Float (single-precision)")))

(event `GuardPatrol`
  (`|AIMoveTo` self (`|GetArrayItem` (`self.PatrolLocation`) (`self.Locations`)) null
    (:`OnSuccess`
      (`KismetSystemLibrary.Delay` 3.0)
      (`self.GuardPatrol`)
      (`/Engine/EditorBlueprintResources/StandardMacros.IncrementInt` (`self.Locations`)
        (:`  `
          (if (== (`self.Locations`) 4)
            (set `self.Locations` 0)))))))

(event `self.PawnSensing.OnSeePawn`
  (params (Pawn :type "Pawn Object Reference"))
  (`KismetSystemLibrary.PrintString` "on see pawn")
  (`|ExecutionSequence`
    (:`then_0`
      (`self.K2_SetActorRotation` (`KismetMathLibrary.FindLookAtRotation` (`self.K2_GetActorLocation`) (`self.K2_GetActorLocation` (`GameplayStatics.GetPlayerPawn` 0))))
      (`|AIMoveTo` self (0.0 0.0 0.0) null))
    (:`then_1`
      (`KismetSystemLibrary.RetriggerableDelay` 1.0)
      (`self.GuardPatrol`))))

(fn `FinishRotation`)

(fn `StartRotating`)

(fn `StopChase`)

(fn `UserConstructionScript`)