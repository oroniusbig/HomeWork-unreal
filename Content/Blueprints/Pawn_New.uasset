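; Pawn that collects weapons and ammo, cycles weapons with Tab and fires impulse-driven BP_Bullet projectiles through a Shoot event.
; BoxCollider overlaps read BPI_Pickupables data, then destroy weapon pickups, or ammo pickups whose weapon type is owned.
; Parallel arrays indexed by the current weapon supply damage, ammo and the material shared by mesh and bullet.
; Weapon pickups append to these arrays even for owned types, and capped ammo pickups use Insert rather than overwriting.
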(event `Shoot`
  (bind _ammo (`self.Ammo`))
  (bind _currentweaponindex (`self.CurrentWeaponIndex`))
  (bind _currentweaponindex_2 (`self.CurrentWeaponIndex`))
  (if (`self.HasWeapon`)
    (if (> (`|GetArrayItem` (`self.Ammo`) (`self.CurrentWeaponIndex`)) 0)
      (bind _returnvalue (`|SpawnActorFromClass` "/Game/Blueprints/BP_Bullet.BP_Bullet_C" (`KismetMathLibrary.MakeTransform` (`SceneComponent.K2_GetComponentLocation` (`self.BarrelPivot`)) (struct) (0.5 0.5 0.5)) "AlwaysSpawn" "MultiplyWithRoot" null null))
      (bind _sphere (`/Game/Blueprints/BP_Bullet.Sphere` _returnvalue))
      (`PrimitiveComponent.SetMaterial` _sphere 0 (`|GetArrayItem` (`self.Materials`) _currentweaponindex_2))
      (`PrimitiveComponent.AddImpulse` _sphere (* (`SceneComponent.GetForwardVector` (`self.BarrelPivot`)) 1000) "None" false)
      (set `/Game/Blueprints/BP_Bullet.Damage` (`|GetArrayItem` (`self.Damage`) _currentweaponindex_2) _returnvalue)
      (bind _result (`/Engine/EditorBlueprintResources/StandardMacros.DecrementInt` (`|GetArrayItem` _ammo _currentweaponindex))
        (:`  `
          (`KismetArrayLibrary.Array_Set` _ammo _currentweaponindex _result)))
      (else
        (`KismetSystemLibrary.PrintString` "no bullets")))))

(event `Key|Tab`
  (params (Key :type "Key Structure"))
  (:`Pressed`
    (if (`self.HasWeapon`)
      (bind _result (`/Engine/EditorBlueprintResources/StandardMacros.IncrementInt` (`self.CurrentWeaponIndex`))
        (:`  `
          (if (>= _result (`KismetArrayLibrary.Array_Length` (`self.WeaponTypes`)))
            (set `self.CurrentWeaponIndex` 0))
          (`PrimitiveComponent.SetMaterial` (`self.SkeletalMesh`) 0 (`|GetArrayItem` (`self.Materials`) (`self.CurrentWeaponIndex`))))))))

(event `self.BoxCollider.OnComponentBeginOverlap`
  (params (OverlappedComponent :type "PrimitiveComponent Object Reference") (OtherActor :type "Actor Object Reference") (OtherComp :type "PrimitiveComponent Object Reference") (OtherBodyIndex :type Integer) (bFromSweep :type Boolean) (SweepResult :type "HitResult Structure (by ref)"))
  (if (`KismetSystemLibrary.DoesImplementInterface` OtherActor "/Game/Blueprints/BPI_Pickupables.BPI_Pickupables_C")
    (bind (_isammo _weapontype _value) (message `/Game/Blueprints/BPI_Pickupables.GetPickupType` OtherActor))
    (if _isammo
      (bind _wasammotaken (`self.AddAmmoType` _weapontype _value))
      (if _wasammotaken
        (`self.K2_DestroyActor` OtherActor :!label _label))
      (else
        (`self.Add Weapon Type` _weapontype _value)
        (goto _label)))))

(fn `Add Weapon Type`
  (params (WeaponType :type "/Game/Blueprints/BPE_WeaponType Enum" :default "NewEnumerator0") (Damage :type Integer))
  (bind _materials (`self.Materials`))
  (if (not (`self.HasWeapon`))
    (set `self.HasWeapon` true)
    (`SceneComponent.SetVisibility` (`self.SkeletalMesh`) true false))
  (`KismetArrayLibrary.Array_Add` (`self.Damage`) Damage)
  (`KismetArrayLibrary.Array_Add` (`self.Ammo`) 5)
  (switch `/Game/Blueprints/BPE_WeaponType` WeaponType
    (:`NewEnumerator0`
      (`KismetArrayLibrary.Array_Add` _materials "/Engine/BasicShapes/BasicShapeMaterial.BasicShapeMaterial"))
    (:`NewEnumerator1`
      (`KismetArrayLibrary.Array_Add` _materials "/Engine/EngineMaterials/EditorBrushMaterial.EditorBrushMaterial")))
  (bind _returnvalue (`KismetArrayLibrary.Array_AddUnique` (`self.WeaponTypes`) WeaponType))
  (bind _output_get (set `self.CurrentWeaponIndex` _returnvalue))
  (`PrimitiveComponent.SetMaterial` (`self.SkeletalMesh`) 0 (`|GetArrayItem` (`self.Materials`) _output_get)))

(fn `AddAmmoType`
  (params (WeaponType :type "/Game/Blueprints/BPE_WeaponType Enum" :default "NewEnumerator0") (AmmoCount :type Integer))
  (returns (WasAmmoTaken :type Boolean))
  (bind _weapontypes (`self.WeaponTypes`))
  (bind _ammo (`self.Ammo`))
  (bind _returnvalue (`KismetArrayLibrary.Array_Find` _weapontypes WeaponType))
  (bind _returnvalue_2 (+ (`|GetArrayItem` _ammo _returnvalue) AmmoCount))
  (if (`KismetArrayLibrary.Array_Contains` _weapontypes WeaponType)
    (if (> _returnvalue_2 50)
      (`KismetArrayLibrary.Array_Insert` _ammo 50 _returnvalue)
      (else
        (`KismetArrayLibrary.Array_Insert` _ammo _returnvalue_2 _returnvalue)))
    (return true)
    (else
      (return false))))

(fn `UserConstructionScript`)