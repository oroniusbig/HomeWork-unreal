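; PC_New is a player controller that turns Enhanced Input actions into player movement, look and shooting, and shows the HUD.
; On BeginPlay it adds the IMC_Override mapping context, and on possess it creates UI_HUD and adds it to the viewport.
; Input events drive the player pawn or character directly for move, inverted-Y look, jump and crouch toggle.
; Shoot casts the pawn to Pawn_New and calls its Shoot function.
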(event `self.ReceiveBeginPlay`
  (`EnhancedInputSubsystemInterface.AddMappingContext` (pcsubsystem `EnhancedInputLocalPlayerSubsystem` self) "/Game/Input/IMC_Override.IMC_Override" 0 (struct)))

(event `EnhancedInput|/Game/Input/IA_NewShoot`
  (params (ActionValue :type Boolean) (ElapsedSeconds :type "Float (double-precision)") (TriggeredSeconds :type "Float (double-precision)") (InputAction :type "InputAction Object Reference" :default "/Game/Input/IA_NewShoot.IA_NewShoot"))
  (:`Triggered`
    (bind _aspawn_new (cast `/Game/Blueprints/Pawn_New` (`GameplayStatics.GetPlayerPawn` 0)))
    (`/Game/Blueprints/Pawn_New.Shoot` _aspawn_new)))

(event `EnhancedInput|/Game/Input/IA_NewMove`
  (params (ActionValue :type "Vector2D Structure") (ElapsedSeconds :type "Float (double-precision)") (TriggeredSeconds :type "Float (double-precision)") (InputAction :type "InputAction Object Reference" :default "/Game/Input/IA_NewMove.IA_NewMove"))
  (bind _returnvalue (`GameplayStatics.GetPlayerPawn` 0))
  (bind (_x _y) (`KismetMathLibrary.BreakVector2D` ActionValue))
  (:`Triggered`
    (`Pawn.AddMovementInput` _returnvalue (`self.GetActorForwardVector` _returnvalue) _x false)
    (`Pawn.AddMovementInput` _returnvalue (`self.GetActorRightVector` _returnvalue) _y false)))

(event `EnhancedInput|/Game/Input/IA_NewJump`
  (params (ActionValue :type Boolean) (ElapsedSeconds :type "Float (double-precision)") (TriggeredSeconds :type "Float (double-precision)") (InputAction :type "InputAction Object Reference" :default "/Game/Input/IA_NewJump.IA_NewJump"))
  (:`Triggered`
    (`Character.Jump` (`GameplayStatics.GetPlayerCharacter` 0))))

(event `EnhancedInput|/Game/Input/IA_NewLook`
  (params (ActionValue :type "Vector2D Structure") (ElapsedSeconds :type "Float (double-precision)") (TriggeredSeconds :type "Float (double-precision)") (InputAction :type "InputAction Object Reference" :default "/Game/Input/IA_NewLook.IA_NewLook"))
  (bind _returnvalue (`GameplayStatics.GetPlayerPawn` 0))
  (:`Triggered`
    (`Pawn.AddControllerPitchInput` _returnvalue (* ActionValue_Y -1.0))
    (`Pawn.AddControllerYawInput` _returnvalue ActionValue_X)))

(event `EnhancedInput|/Game/Input/IA_NewCrouch`
  (params (ActionValue :type Boolean) (ElapsedSeconds :type "Float (double-precision)") (TriggeredSeconds :type "Float (double-precision)") (InputAction :type "InputAction Object Reference" :default "/Game/Input/IA_NewCrouch.IA_NewCrouch"))
  (bind _returnvalue (`GameplayStatics.GetPlayerCharacter` 0))
  (:`Triggered`
    (if (`NavMovementComponent.IsCrouching` (`Character.CharacterMovement` _returnvalue))
      (`Character.UnCrouch` _returnvalue)
      (else
        (`Character.Crouch` _returnvalue)))))

(event `self.ReceivePossess`
  (params (PossessedPawn :type "Pawn Object Reference"))
  (bind _returnvalue (`|CreateWidget` "/Game/Blueprints/UI/UI_HUD.UI_HUD_C" self))
  (`UserWidget.AddToViewport` _returnvalue 0))

(fn `UserConstructionScript`)