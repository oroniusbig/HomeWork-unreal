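; Enemy guard that patrols, spots the player and gives chase, driven by a Patrolling/Staring/Chasing state switch in ChangeState.
; Patrol cycles four locations with AIMoveTo; Tick line-traces from the head when the player is inside the Collider, triggering Staring on sight.
; Staring halts movement for three seconds before chasing or resuming patrol; chases revert after three seconds.
; Damage lowers HP and destroys the guard below zero; RotateTowardPlayer is an empty stub.
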(event `Patrol`
  (`|AIMoveTo` self (`|GetArrayItem` (`self.PatrolLocations`) (`self.Locations`)) null
    (:`OnSuccess`
      (`self.Patrol`)
      (`/Engine/EditorBlueprintResources/StandardMacros.IncrementInt` (`self.Locations`)
        (:`  `
          (if (== (`self.Locations`) 4)
            (set `self.Locations` 0)))))))

(event `self.ReceiveBeginPlay`
  (`self.ChangeState` "NewEnumerator0"))

(event `Chase`
  (`|AIMoveTo` self (0.0 0.0 0.0) (`GameplayStatics.GetPlayerPawn` 0)
    (:`then`
      (`KismetSystemLibrary.Delay` 3.0)
      (`self.ChangeState` "NewEnumerator0"))
    (:`OnSuccess`
      (`KismetSystemLibrary.PrintString` "ded" true true (struct :`R` 1.0 :`G` 0.001821 :`B` 0.001821 :`A` 1.0) 30.0))))

(event `Stare`
  (`Controller.StopMovement` (`AIBlueprintHelperLibrary.GetAIController` self))
  (`KismetSystemLibrary.Delay` 3.0)
  (if (`self.PlayerInRange`)
    (`self.ChangeState` "NewEnumerator1")
    (else
      (`self.ChangeState` "NewEnumerator0"))))

(event `self.ReceiveTick`
  (params (DeltaSeconds :type "Float (single-precision)"))
  (`|ExecutionSequence`
    (:`then_0`
      (if (`|EnumEquality` (`self.State`) "NewEnumerator5")
        (`self.RotateTowardPlayer`)))
    (:`then_1`
      (if (and (`self.PlayerInRange`) (`|EnumEquality` (`self.State`) "NewEnumerator0"))
        (bind _outhit (`KismetSystemLibrary.LineTraceSingle` :`Start` (`SceneComponent.K2_GetComponentLocation` (`self.HeadPivot`)) :`End` (`self.K2_GetActorLocation` (`GameplayStatics.GetPlayerPawn` 0)) :`TraceChannel` "TraceTypeQuery1" :`DrawDebugType` "Persistent"))
        (if (== (`.HitActor` (`GameplayStatics.BreakHitResult` _outhit)) (`GameplayStatics.GetPlayerPawn` 0))
          (`self.ChangeState` "NewEnumerator5"))))))

(event `self.Collider.OnComponentBeginOverlap`
  (params (OverlappedComponent :type "PrimitiveComponent Object Reference") (OtherActor :type "Actor Object Reference") (OtherComp :type "PrimitiveComponent Object Reference") (OtherBodyIndex :type Integer) (bFromSweep :type Boolean) (SweepResult :type "HitResult Structure (by ref)"))
  (if (== OtherActor (`GameplayStatics.GetPlayerPawn` 0))
    (set `self.PlayerInRange` true)))

(event `self.Collider.OnComponentEndOverlap`
  (params (OverlappedComponent :type "PrimitiveComponent Object Reference") (OtherActor :type "Actor Object Reference") (OtherComp :type "PrimitiveComponent Object Reference") (OtherBodyIndex :type Integer))
  (if (== OtherActor (`GameplayStatics.GetPlayerPawn` 0))
    (set `self.PlayerInRange` false)))

(event `/Game/Blueprints/BPI_NewHitable.TakeDamage`
  (params (Damage :type Integer))
  (bind _hp (`self.HP`))
  (set `self.HP` (- _hp Damage))
  (`KismetSystemLibrary.PrintString` (`KismetStringLibrary.Conv_IntToString` _hp) true true (struct :`R` 0.217874 :`G` 1.0 :`A` 1.0) 500.0)
  (if (< (`self.HP`) 0)
    (set `self.HP` 0)
    (`KismetSystemLibrary.PrintString` "Enemy Dead")
    (`self.K2_DestroyActor`)))

(fn `ChangeState`
  (params (NewState :type "/Game/Blueprints/AI/AI_States Enum" :default "NewEnumerator0"))
  (if (`|EnumInequality` NewState (`self.State`))
    (bind _output_get (set `self.State` NewState))
    (switch `/Game/Blueprints/AI/AI_States` _output_get
      (:`NewEnumerator0`
        (`self.Patrol`))
      (:`NewEnumerator1`
        (`self.Chase`))
      (:`NewEnumerator5`
        (`self.Stare`)))))

(fn `RotateTowardPlayer`)

(fn `UserConstructionScript`)