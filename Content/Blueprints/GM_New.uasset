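; GM_New, apparently a game mode, scatters white and red mag actors across random BP_SpawnPoint locations when play begins.
; SpawnWhiteMags runs first, then SpawnRedMags, each gathering the existing spawn points and placing a fixed batch.
; Each used point is removed from the array and destroyed, so red mags only get locations the white ones left free.
; Leftover debug-print and single-spawn nodes in the event graph never run.
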(event `self.ReceiveBeginPlay`
  (`self.SpawnWhiteMags`)
  (`self.SpawnRedMags`))

(fn `SpawnRedMags`
  (locals (`Spawn Refs` :type "Array of /Game/Blueprints/BP_SpawnPoint Object Reference") (`Local Item` :type "/Game/Blueprints/BP_SpawnPoint Object Reference"))
  (bind _outactors (`GameplayStatics.GetAllActorsOfClass` "/Game/Blueprints/BP_SpawnPoint.BP_SpawnPoint_C"))
  (set `local.Spawn Refs` _outactors)
  (for _ (range 8)
    (set `local.Local Item` (`KismetArrayLibrary.Array_Random` (`local.Spawn Refs`)))
    (`|SpawnActorFromClass` "/Game/Blueprints/BP_RedMag.BP_RedMag_C" (`KismetMathLibrary.MakeTransform` (`self.K2_GetActorLocation` (`local.Local Item`))) "Undefined" "MultiplyWithRoot" null null)
    (`KismetArrayLibrary.Array_RemoveItem` (`local.Spawn Refs`) (`local.Local Item`))
    (`self.K2_DestroyActor` (`local.Local Item`))))

(fn `SpawnWhiteMags`
  (locals (`Spawn Refs` :type "Array of /Game/Blueprints/BP_SpawnPoint Object Reference") (`Local Item` :type "/Game/Blueprints/BP_SpawnPoint Object Reference"))
  (bind _outactors (`GameplayStatics.GetAllActorsOfClass` "/Game/Blueprints/BP_SpawnPoint.BP_SpawnPoint_C"))
  (set `local.Spawn Refs` _outactors)
  (for _ (range 8)
    (set `local.Local Item` (`KismetArrayLibrary.Array_Random` (`local.Spawn Refs`)))
    (`|SpawnActorFromClass` "/Game/Blueprints/BP_WhiteMag.BP_WhiteMag_C" (`KismetMathLibrary.MakeTransform` (`self.K2_GetActorLocation` (`local.Local Item`))) "Undefined" "MultiplyWithRoot" null null)
    (`KismetArrayLibrary.Array_RemoveItem` (`local.Spawn Refs`) (`local.Local Item`))
    (`self.K2_DestroyActor` (`local.Local Item`))))

(fn `UserConstructionScript`)